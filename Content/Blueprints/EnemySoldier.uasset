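; EnemySoldier is an enemy actor that takes damage, shoots at the player and awards score when killed.
; Damage plays a hurt sound and lowers Health; at zero, a DoOnce adds score to the game instance, ragdolls the body, removes the gun and destroys the actor after a delay.
; The ShootPlayer event spawns a bullet at the fire point aimed at the player, and is skipped once the body simulates physics.
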(event `self.ReceiveAnyDamage`
  (params (Damage :type "Float (single-precision)") (DamageType :type "DamageType Object Reference") (InstigatedBy :type "Controller Object Reference") (DamageCauser :type "Actor Object Reference"))
  (bind _aswi_ggame_instance (cast `/Game/GameModes/WiGGameInstance` (`GameplayStatics.GetGameInstance`) :!pure true))
  ;[1 1 1] Health, damage, death
  (`GameplayStatics.PlaySoundAtLocation` "/Game/Audio/Hurt.Hurt" (`self.K2_GetActorLocation`) (struct) 1.0 1.0 0.0 null null null)
  (set `self.Health` (- (`self.Health`) Damage))
  (if (<= (`self.Health`) 0.0)
    (`/Engine/EditorBlueprintResources/StandardMacros.DoOnce` false
      (:`Completed`
        (set `/Game/GameModes/WiGGameInstance.Score` (+ (`/Game/GameModes/WiGGameInstance.Score` _aswi_ggame_instance) 100.0) _aswi_ggame_instance)
        (`PrimitiveComponent.SetSimulatePhysics` (`self.Body`) true)
        (`ActorComponent.K2_DestroyComponent` (`self.Gun`))
        (`KismetSystemLibrary.Delay` 2.0)
        (`self.K2_DestroyActor`)))
    (else
      (`GameplayStatics.SpawnEmitterAtLocation` null))))

(event `Shoot Player`
  (params (TargetToShoot :type "Actor Object Reference"))
  ;[1 1 1] AI
  (if (not (`SceneComponent.IsSimulatingPhysics` (`self.Body`) "None"))
    (`|SpawnActorFromClass` "/Game/Blueprints/Bullet.Bullet_C" (`KismetMathLibrary.MakeTransform` (+ (`SceneComponent.K2_GetComponentLocation` (`self.FirePoint`)) (`KismetMathLibrary.GreaterGreater_VectorRotator` (`self.GunOffset`) (`SceneComponent.K2_GetComponentRotation` (`self.Gun`)))) (`KismetMathLibrary.FindLookAtRotation` (`self.K2_GetActorLocation`) (`self.K2_GetActorLocation` (cast `/Game/Blueprints/Player1` (`GameplayStatics.GetPlayerCharacter` 0) :!pure true)))) "Undefined" "OverrideRootScale" null null)
    (`GameplayStatics.PlaySoundAtLocation` "/Game/Audio/Gunshot2.Gunshot2" (`self.K2_GetActorLocation`) (struct) 1.0 1.0 0.0 null null null)))

(fn `UserConstructionScript`)