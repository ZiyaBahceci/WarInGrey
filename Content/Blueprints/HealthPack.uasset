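; HealthPack is a pickup actor that restores a player's health when touched.
; Its Box overlap casts the other actor to Player1, then either adds a fixed amount at lower health or tops up to 100.
; After healing it passes the new value to the player's CallUpdateUI and destroys itself, staying in the world if health is already full.
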(event `self.Box.OnComponentBeginOverlap`
  (params (OverlappedComponent :type "PrimitiveComponent Object Reference") (OtherActor :type "Actor Object Reference") (OtherComp :type "PrimitiveComponent Object Reference") (OtherBodyIndex :type Integer) (bFromSweep :type Boolean) (SweepResult :type "HitResult Structure (by ref)"))
  ;[1 1 1] Add health to player. If player health is less than or equal to 60, add 40 health. If player health is above 60, fill health up to 100. If above 100, don't touch.
  (bind _asplayer_1 (cast `/Game/Blueprints/Player1` OtherActor))
  (if (<= (`/Game/Blueprints/Player1.Health` _asplayer_1) 60.0)
    (bind _output_get (set `/Game/Blueprints/Player1.Health` (+ (`/Game/Blueprints/Player1.Health` _asplayer_1) 40.0) _asplayer_1))
    (`/Game/Blueprints/Player1.UpdateUI` _asplayer_1 _output_get)
    (`self.K2_DestroyActor`)
    (elif (< (`/Game/Blueprints/Player1.Health` _asplayer_1) 100.0)
      (bind _output_get_2 (set `/Game/Blueprints/Player1.Health` 100.0 _asplayer_1))
      (`/Game/Blueprints/Player1.UpdateUI` _asplayer_1 _output_get_2)
      (`self.K2_DestroyActor`))))

(fn `UserConstructionScript`)