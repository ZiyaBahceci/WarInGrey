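; Factory gate Blueprint that shuts behind the player as a scripted story beat and checkpoint.
; When the player enters the trigger box, the gate slides shut with a sound, the objective and marker update, and the box is destroyed.
; The overlap also saves checkpoint location and gate state to the game instance.
; Tick reads that state every frame and, if set, snaps the gate to its closed position and removes the trigger.
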(event `self.ReceiveTick`
  (params (DeltaSeconds :type "Float (single-precision)"))
  ;[1 1 1] Is gate opened pre-checkpoint?
  (if (`/Game/GameModes/WiGGameInstance.GateClosed` (cast `/Game/GameModes/WiGGameInstance` (`GameplayStatics.GetGameInstance`) :!pure true))
    ;[1 1 1] Open gate
    (`KismetSystemLibrary.MoveComponentTo` (`self.Gate1`) (904.0 0.0 0.0) (struct) false false 0.0)
    (`ActorComponent.K2_DestroyComponent` (`self.Box`))))

(event `self.Box.OnComponentBeginOverlap`
  (params (OverlappedComponent :type "PrimitiveComponent Object Reference") (OtherActor :type "Actor Object Reference") (OtherComp :type "PrimitiveComponent Object Reference") (OtherBodyIndex :type Integer) (bFromSweep :type Boolean) (SweepResult :type "HitResult Structure (by ref)"))
  (cast `/Game/Blueprints/BP_Player1` OtherActor)
  (`KismetSystemLibrary.MoveComponentTo` (`self.Gate1`) (904.0 0.0 0.0) (struct) false false 0.25)
  (bind _asplayer_1 (cast `/Game/Blueprints/BP_Player1` (`GameplayStatics.GetPlayerCharacter` 0)))
  (set `/Game/Blueprints/BP_Player1.ObjectiveText` "They closed the gates. Go to the security room to open ventilation shaft door" _asplayer_1)
  (`GameplayStatics.PlaySoundAtLocation` "/Game/Audio/GateClose.GateClose" (`self.K2_GetActorLocation`) (struct) 1.0 1.0 0.0 null null null)
  (`ActorComponent.K2_DestroyComponent` (`self.Box`))
  (bind _asplayer_1_2 (cast `/Game/Blueprints/BP_Player1` (`GameplayStatics.GetPlayerCharacter` 0)))
  (set `/Game/Blueprints/BP_Player1.GateIsClosed` true _asplayer_1_2)
  (bind _aswi_ggame_instance (cast `/Game/GameModes/WiGGameInstance` (`GameplayStatics.GetGameInstance`)))
  (set `/Game/GameModes/WiGGameInstance.MarkerLocation` (8953.0 2713.0 209.0) _aswi_ggame_instance)
  (`/Engine/EditorBlueprintResources/StandardMacros.DoOnce` false
    (:`Completed`
      (bind _aswi_ggame_instance_2 (cast `/Game/GameModes/WiGGameInstance` (`GameplayStatics.GetGameInstance`)))
      (set `/Game/GameModes/WiGGameInstance.CheckpointSaved` true _aswi_ggame_instance_2)
      (set `/Game/GameModes/WiGGameInstance.SavedLocation` (7090.0 -2096.0 11.0) _aswi_ggame_instance_2)
      (`KismetSystemLibrary.PrintString` "checkpoint saved")
      (set `/Game/GameModes/WiGGameInstance.GateClosed` true _aswi_ggame_instance_2)
      (set `/Game/GameModes/WiGGameInstance.InCompound` true _aswi_ggame_instance_2))))

(fn `UserConstructionScript`)