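; A locked, hinged door Blueprint that the player opens and closes with F once their Player1 character has the key.
; DoorTrigger overlap toggles input on the door, and InteractState chooses whether DoorTimeline plays or reverses, swinging the root's yaw toward Angle with sweep enabled.
; Without the key, it sets the player's warehouse hint text and, through a never-reset DoOnce, shows a Hint widget once for five seconds.
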(event `self.DoorTrigger.OnComponentBeginOverlap`
  (params (OverlappedComponent :type "PrimitiveComponent Object Reference") (OtherActor :type "Actor Object Reference") (OtherComp :type "PrimitiveComponent Object Reference") (OtherBodyIndex :type Integer) (bFromSweep :type Boolean) (SweepResult :type "HitResult Structure (by ref)"))
  ;[1 1 1] Door Proximity
  (`self.EnableInput` (`GameplayStatics.GetPlayerController` 0)))

(event `self.DoorTrigger.OnComponentEndOverlap`
  (params (OverlappedComponent :type "PrimitiveComponent Object Reference") (OtherActor :type "Actor Object Reference") (OtherComp :type "PrimitiveComponent Object Reference") (OtherBodyIndex :type Integer))
  ;[1 1 1] Door Proximity
  (`self.DisableInput` (`GameplayStatics.GetPlayerController` 0)))

(event `Key|F`
  (params (Key :type "Key Structure"))
  ;[1 1 1] Check if player has key
  (:`Pressed`
    (bind _asplayer_1 (cast `/Game/Blueprints/Player1` (`GameplayStatics.GetPlayerCharacter` 0)))
    (if (`/Game/Blueprints/Player1.HasKey` _asplayer_1)
      ;[1 1 1] Open/Close Door
      (if (`self.InteractState`)
        (set `self.InteractState` false)
        (bind (_direction _doorinterpolation) (`Timeline|DoorTimeline` :!via `Reverse` :!label _label)
          (:`Update`
            (`SceneComponent.K2_SetRelativeRotation` (`self.DefaultSceneRoot`) (`KismetMathLibrary.MakeRotator` 0.0 0.0 (* (`self.Angle`) _doorinterpolation)) true false)))
        (else
          (set `self.InteractState` true)
          (goto _label)))
      (else
        ;[1 1 1] If player doesn't have the key, create hint widget for 5 seconds.
        (bind _asplayer_1_2 (cast `/Game/Blueprints/Player1` (`GameplayStatics.GetPlayerCharacter` 0)))
        (set `/Game/Blueprints/Player1.HintText` "Door is locked. Key is most likely in the warehouse." _asplayer_1_2)
        (`/Engine/EditorBlueprintResources/StandardMacros.DoOnce` false
          (:`Completed`
            (bind _returnvalue (`|CreateWidget` "/Game/UI/Hint.Hint_C" (`GameplayStatics.GetPlayerController` 0)))
            (`UserWidget.AddToViewport` _returnvalue 0)
            (`KismetSystemLibrary.Delay` 5.0)
            (`Widget.RemoveFromParent` _returnvalue)))))))

(fn `UserConstructionScript`)