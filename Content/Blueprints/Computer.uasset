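; Interactive computer Blueprint that opens the topside ventilation shaft so the player can enter the factory.
; A box overlap enables or disables player input, letting a one-time F press swap the Closed and Open screen displays.
; That press also sets the player's opened flag and objective text, moves the objective marker, and saves a hardcoded checkpoint with progress flags to the game instance.
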(event `self.Box.OnComponentBeginOverlap`
  (params (OverlappedComponent :type "PrimitiveComponent Object Reference") (OtherActor :type "Actor Object Reference") (OtherComp :type "PrimitiveComponent Object Reference") (OtherBodyIndex :type Integer) (bFromSweep :type Boolean) (SweepResult :type "HitResult Structure (by ref)"))
  ;[1 1 1] Enable/Disable input
  (`self.EnableInput` (`GameplayStatics.GetPlayerController` 0)))

(event `self.Box.OnComponentEndOverlap`
  (params (OverlappedComponent :type "PrimitiveComponent Object Reference") (OtherActor :type "Actor Object Reference") (OtherComp :type "PrimitiveComponent Object Reference") (OtherBodyIndex :type Integer))
  ;[1 1 1] Enable/Disable input
  (`self.DisableInput` (`GameplayStatics.GetPlayerController` 0)))

(event `Key|F`
  (params (Key :type "Key Structure"))
  (:`Pressed`
    (`/Engine/EditorBlueprintResources/StandardMacros.DoOnce` false
      (:`Completed`
        ;[1 1 1] Change text on computer
        (`SceneComponent.SetVisibility` (`self.Closed`) false false)
        (`SceneComponent.SetVisibility` (`self.Open`) true false)
        ;[1 1 1] Open topside ventilation gates/update player objective accordingly
        (bind _asplayer_1 (cast `/Game/Blueprints/Player1` (`GameplayStatics.GetPlayerCharacter` 0)))
        (set `/Game/Blueprints/Player1.TopsideOpened` true _asplayer_1)
        (set `/Game/Blueprints/Player1.ObjectiveText` "Ventilation shaft is open. Enter the factory." _asplayer_1)
        ;[1 1 1] Set Marker New Location
        (bind _aswi_ggame_instance (cast `/Game/GameModes/WiGGameInstance` (`GameplayStatics.GetGameInstance`)))
        (set `/Game/GameModes/WiGGameInstance.MarkerLocation` (8415.0 2987.0 2015.0) _aswi_ggame_instance)
        ;[1 1 1] Save last player location
        (bind _aswi_ggame_instance_2 (cast `/Game/GameModes/WiGGameInstance` (`GameplayStatics.GetGameInstance`)))
        (set `/Game/GameModes/WiGGameInstance.CheckpointSaved` true _aswi_ggame_instance_2)
        (set `/Game/GameModes/WiGGameInstance.SavedLocation` (9300.0 2411.0 103.0) _aswi_ggame_instance_2)
        (`KismetSystemLibrary.PrintString` "checkpoint saved")
        ;[1 1 1] Save-Related Booleans
        (set `/Game/GameModes/WiGGameInstance.InSecurityRoom` true _aswi_ggame_instance_2)
        (set `/Game/GameModes/WiGGameInstance.GateClosed` true _aswi_ggame_instance_2)
        (set `/Game/GameModes/WiGGameInstance.InCompound` true _aswi_ggame_instance_2)))))

(fn `UserConstructionScript`)