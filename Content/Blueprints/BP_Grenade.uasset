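; Grenade actor that plays a launch sound on spawn and explodes when it overlaps another actor.
; Each overlap makes a direct-hit damage call naming the other actor as causer with no target set, starts a short lifespan, enables physics and spawns BP_Explosion.
; A DoOnce then limits the explosion sound and radial splash damage, found by sphere overlap on pawns and physics bodies, to the first overlap.
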(event `self.ReceiveBeginPlay`
  (`GameplayStatics.PlaySoundAtLocation` "/Game/Audio/GrenadeLaunch.GrenadeLaunch" (`self.K2_GetActorLocation`) (struct) 1.0 1.0 0.0 null null null))

(event `self.ReceiveActorBeginOverlap`
  (params (OtherActor :type "Actor Object Reference"))
  (bind _returnvalue (`self.K2_GetActorLocation`))
  ;[1 1 1] Direct hit damage
  (`GameplayStatics.ApplyDamage` null 20.0 null OtherActor)
  (`self.SetLifeSpan` 3.0)
  (`PrimitiveComponent.SetSimulatePhysics` (`self.Grenade`) true)
  (`SceneComponent.ToggleVisibility` (`self.Explosion`) false)
  ;[1 1 1] Explosion & Splash Damage
  (`|SpawnActorFromClass` "/Game/Blueprints/BP_Explosion.BP_Explosion_C" (`KismetMathLibrary.MakeTransform` (`self.K2_GetActorLocation`)) "Undefined" "OverrideRootScale" null null)
  (`/Engine/EditorBlueprintResources/StandardMacros.DoOnce` false
    (:`Completed`
      (`GameplayStatics.PlaySoundAtLocation` "/Game/Audio/Explosion.Explosion" _returnvalue (struct) 1.0 1.0 0.0 null null null)
      (bind (_outactors _returnvalue_2) (`KismetSystemLibrary.SphereOverlapActors` _returnvalue 300.0 (`|MakeArray` "ObjectTypeQuery3" "ObjectTypeQuery4" :!type "EObjectTypeQuery Enum")))
      (if _returnvalue_2
        (for _array_element _outactors
          (`GameplayStatics.ApplyDamage` _array_element 60.0))))))

(fn `UserConstructionScript`)