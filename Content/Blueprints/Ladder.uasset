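; Climbable ladder actor whose length follows the EndOfLadder vector's magnitude.
; The construction script stacks child actor pieces downward at PieceSize intervals and fits the Box trigger to that length plus Offset.
; Box overlaps call ClimbLadder and LeaveLadder on Player1.
; The box scales up horizontally on entry and shrinks on exit, so the exit boundary sits wider than the entry one.
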(event `self.Box.OnComponentBeginOverlap`
  (params (OverlappedComponent :type "PrimitiveComponent Object Reference") (OtherActor :type "Actor Object Reference") (OtherComp :type "PrimitiveComponent Object Reference") (OtherBodyIndex :type Integer) (bFromSweep :type Boolean) (SweepResult :type "HitResult Structure (by ref)"))
  ;[1 1 1] When player enters the box collider, increase box collider size.
  (bind _asplayer_1 (cast `/Game/Blueprints/Player1` OtherActor))
  (`SceneComponent.SetRelativeScale3D` (`self.Box`) (2.5 1.8 1.0))
  (`/Game/Blueprints/Player1.ClimbLadder` _asplayer_1))

(event `self.Box.OnComponentEndOverlap`
  (params (OverlappedComponent :type "PrimitiveComponent Object Reference") (OtherActor :type "Actor Object Reference") (OtherComp :type "PrimitiveComponent Object Reference") (OtherBodyIndex :type Integer))
  ;[1 1 1] When player leaves ladder, reset the box collider size.
  (bind _asplayer_1 (cast `/Game/Blueprints/Player1` OtherActor))
  (`SceneComponent.SetRelativeScale3D` (`self.Box`) (0.75 0.5 1.0))
  (`/Game/Blueprints/Player1.LeaveLadder` _asplayer_1))

(fn `UserConstructionScript`
  (bind _box (`self.Box`))
  (bind _returnvalue (/ (+ (`KismetMathLibrary.VSize` (`self.EndOfLadder`)) (`self.Offset`)) 2.0))
  (for _index (range (+ (`.ReturnValue` (`KismetMathLibrary.FMod` (`KismetMathLibrary.VSize` (`self.EndOfLadder`)) (`self.PieceSize`))) 1))
    (`AddComponent|NODE_AddChildActorComponent-0` :`RelativeTransform` (`KismetMathLibrary.MakeTransform` (`KismetMathLibrary.MakeVector` 0.0 15.0 (* -1 (* _index (`self.PieceSize`)))))))
  (`BoxComponent.SetBoxExtent` _box (`KismetMathLibrary.MakeVector` 75.0 90.0 _returnvalue) true)
  (`SceneComponent.K2_SetRelativeLocation` _box (`KismetMathLibrary.MakeVector` 0.0 40.0 (+ (* _returnvalue -1.0) (`self.Offset`))) false false))