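; Behavior tree task that picks a search point for a soldier AI looking for its enemy.
; On execute it averages the Enemy actor's actual current position with the blackboard LastSeenLocation, so the search is biased toward where the enemy really is.
; It writes a random navigable point within a fixed radius of that midpoint to SearchLocation and always finishes successfully.
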(event `self.ReceiveExecuteAI`
  (params (OwnerController :type "AIController Object Reference") (ControlledPawn :type "Pawn Object Reference"))
  (bind _returnvalue (`AIBlueprintHelperLibrary.GetBlackboard` OwnerController))
  (`BlackboardComponent.SetValueAsVector` _returnvalue "SearchLocation" (`NavigationSystemV1.K2_GetRandomLocationInNavigableRadius` (/ (+ (`Actor.K2_GetActorLocation` (cast `Actor` (`BlackboardComponent.GetValueAsObject` _returnvalue "Enemy") :!pure true)) (`BlackboardComponent.GetValueAsVector` _returnvalue "LastSeenLocation")) 2.0) 3000.0 null null))
  (`self.FinishExecute` true))