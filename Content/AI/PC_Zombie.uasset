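; PC_Zombie is the zombie AI controller, which starts the BT_Zombie behavior tree on BeginPlay.
; On AI perception updates for BP_Player1, it writes whether the player is currently sensed to the HasSpottedPlayer blackboard key.
; The first such update, sensed or lost, also plays a detection cue at the world origin through a DoOnce that is never reset.
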(event `self.ReceiveBeginPlay`
  (`self.RunBehaviorTree` "/Game/AI/BT_Zombie.BT_Zombie"))

(event `self.AIPerception.OnTargetPerceptionUpdated`
  (params (Actor :type "Actor Object Reference") (Stimulus :type "AIStimulus Structure"))
  (set `self.HasSensed` (`.bSuccessfullySensed` (break `AIStimulus` Stimulus)))
  (cast `/Game/Blueprints/BP_Player1` Actor)
  (`BlackboardComponent.SetValueAsBool` (`AIBlueprintHelperLibrary.GetBlackboard` null) "HasSpottedPlayer" (`self.HasSensed`))
  (`/Engine/EditorBlueprintResources/StandardMacros.DoOnce` false
    (:`Completed`
      (`GameplayStatics.PlaySoundAtLocation` "/Game/Audio/ZombieDetectCue.ZombieDetectCue" (0.0 0.0 0.0) (struct) 1.0 1.0 0.0 null null null))))

(fn `UserConstructionScript`)