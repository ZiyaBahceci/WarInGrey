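; AI controller for soldier enemies that runs the soldier behavior tree and blackboard on possess.
; On begin play it caches the first player character as its Enemy and writes it to the blackboard.
; Perception updates for that actor set CanSeePlayer from its first stimulus, and store the player's current location as LastSeenLocation when sensing fails.
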(event `self.ReceivePossess`
  (params (PossessedPawn :type "Pawn Object Reference"))
  (`self.UseBlackboard` "/Game/AI/BB_Soldier.BB_Soldier")
  (`self.RunBehaviorTree` "/Game/AI/BT_Soldier.BT_Soldier"))

(event `self.ReceiveBeginPlay`
  (bind _returnvalue (`GameplayStatics.GetPlayerCharacter` 0))
  (set `self.Enemy` _returnvalue)
  (`BlackboardComponent.SetValueAsObject` (`AIBlueprintHelperLibrary.GetBlackboard` null) "Enemy" _returnvalue))

(event `self.AIPerception.OnPerceptionUpdated`
  (params (UpdatedActors :type "Array of Actor Object Reference (by ref)"))
  (bind _returnvalue (`AIBlueprintHelperLibrary.GetBlackboard` null))
  (for _array_element UpdatedActors
    (if (== _array_element (`self.Enemy`))
      (bind _info (`AIPerceptionComponent.GetActorsPerception` (`self.AIPerception`) _array_element))
      (bind (_age _expirationage _strength _stimuluslocation _receiverlocation _tag _bsuccessfullysensed) (break `AIStimulus` (`|GetArrayItem` (`.LastSensedStimuli` (break `ActorPerceptionBlueprintInfo` _info)))))
      (`BlackboardComponent.SetValueAsBool` _returnvalue "CanSeePlayer" _bsuccessfullysensed)
      (if (not _bsuccessfullysensed)
        (`BlackboardComponent.SetValueAsVector` _returnvalue "LastSeenLocation" (`self.K2_GetActorLocation` (`self.Enemy`)))))))

(fn `UserConstructionScript`)