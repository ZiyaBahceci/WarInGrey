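; Officer boss enemy whose death, while the player is alive, awards score and ends the level by opening Endgame.
; Pawn sensing drives simple AI that approaches the player, then fires bullets and cooldown-limited grenades.
; Damage updates the boss health widget and draws the officer toward the player, or on death turns body parts to physics and destroys the gun.
; A per-tick line trace shows the health bar only with clear line of sight.
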(event `self.ReceiveBeginPlay`
  ;[1 1 1] Boss Health UI
  (bind _asplayer_1 (cast `/Game/Blueprints/Player1` (`GameplayStatics.GetPlayerCharacter` 0)))
  (set `self.PlayerReference` _asplayer_1)
  (bind _asboss_health_ui (cast `/Game/UI/BossHealthUI` (`WidgetComponent.GetUserWidgetObject` (`self.HealthBar`))))
  (bind _output_get (set `self.HealthWidgetRef` _asboss_health_ui))
  (set `/Game/UI/BossHealthUI.Health` 600.0 _output_get))

(event `self.ReceiveTick`
  (params (DeltaSeconds :type "Float (single-precision)"))
  (bind (_returnvalue_x _returnvalue_y _returnvalue_z) (`KismetMathLibrary.BreakVector` (`self.K2_GetActorLocation`)))
  (bind (_returnvalue_x_2 _returnvalue_y_2 _returnvalue_z_2) (`KismetMathLibrary.BreakVector` (`self.K2_GetActorLocation` (`GameplayStatics.GetPlayerCharacter` 0))))
  ;[1 1 1] Boss Health UI
  (bind _outhit (`KismetSystemLibrary.LineTraceSingleForObjects` (`KismetMathLibrary.MakeVector` _returnvalue_x _returnvalue_y (+ _returnvalue_z 44.0)) (`KismetMathLibrary.MakeVector` _returnvalue_x_2 _returnvalue_y_2 (+ _returnvalue_z_2 44.0)) (`|MakeArray` "ObjectTypeQuery3" "ObjectTypeQuery1" "ObjectTypeQuery2" "ObjectTypeQuery4" :!type "EObjectTypeQuery Enum")))
  (if (== (`.HitActor` (`GameplayStatics.BreakHitResult` _outhit)) (`GameplayStatics.GetPlayerCharacter` 0))
    (`SceneComponent.SetVisibility` (`self.HealthBar`) true false)
    (else
      (`SceneComponent.SetVisibility` (`self.HealthBar`) false false))))

(event `self.ReceiveAnyDamage`
  (params (Damage :type "Float (single-precision)") (DamageType :type "DamageType Object Reference") (InstigatedBy :type "Controller Object Reference") (DamageCauser :type "Actor Object Reference"))
  (bind _aswi_ggame_instance (cast `/Game/GameModes/WiGGameInstance` (`GameplayStatics.GetGameInstance`) :!pure true))
  ;[1 1 1] Health, Damage, Death
  (bind _output_get (set `self.Health` (- (`self.Health`) Damage)))
  (set `/Game/UI/BossHealthUI.Health` _output_get (`self.HealthWidgetRef`))
  (if (<= (`self.Health`) 0.0)
    (bind _asplayer_1 (cast `/Game/Blueprints/Player1` (`GameplayStatics.GetPlayerCharacter` 0)))
    (if (> (`/Game/Blueprints/Player1.Health` _asplayer_1) 0.0)
      (set `/Game/GameModes/WiGGameInstance.Score` (+ (`/Game/GameModes/WiGGameInstance.Score` _aswi_ggame_instance) 500.0) _aswi_ggame_instance)
      (`PrimitiveComponent.SetSimulatePhysics` (`self.Body`) true)
      (`PrimitiveComponent.SetSimulatePhysics` (`self.LeftArmLower`) true)
      (`PrimitiveComponent.SetSimulatePhysics` (`self.LeftArmUpper`) true)
      (`PrimitiveComponent.SetSimulatePhysics` (`self.RightLeg`) true)
      (`PrimitiveComponent.SetSimulatePhysics` (`self.LeftLeg`) true)
      (`PrimitiveComponent.SetSimulatePhysics` (`self.Neck`) true)
      (`PrimitiveComponent.SetSimulatePhysics` (`self.Head`) true)
      (`PrimitiveComponent.SetSimulatePhysics` (`self.RightArmUpper`) true)
      (`PrimitiveComponent.SetSimulatePhysics` (`self.RightArmLower`) true)
      (`ActorComponent.K2_DestroyComponent` (`self.Gun`))
      (set `/Game/Blueprints/Player1.ObjectiveText` "Officer is dead! Level ends in 5 seconds." _asplayer_1)
      (bind _asboss_health_ui (cast `/Game/UI/BossHealthUI` (`WidgetComponent.GetUserWidgetObject` (`self.HealthBar`))))
      (`Widget.SetVisibility` _asboss_health_ui "Hidden")
      (`KismetSystemLibrary.Delay` 5.0)
      (`self.K2_TeleportTo` :`self` _asplayer_1 :`DestLocation` (-2839.0 -350.0 12500.0))
      (`WidgetLayoutLibrary.RemoveAllWidgets`)
      (set `/Game/Blueprints/Player1.GameOver` true _asplayer_1)
      (`GameplayStatics.OpenLevel` "Endgame"))
    (else
      (bind _asplayer_1_2 (cast `/Game/Blueprints/Player1` (`GameplayStatics.GetPlayerCharacter` 0)))
      (`|AIMoveTo` self (0.0 0.0 0.0) _asplayer_1_2 750.0))))

(event `self.PawnSensing.OnSeePawn`
  (params (Pawn :type "Pawn Object Reference"))
  ;[1 1 1] AI (Simpler AI to make it easier to fight)
  (bind _asplayer_1 (cast `/Game/Blueprints/Player1` Pawn))
  (set `self.CanSeePlayer` true)
  (`|AIMoveTo` self (0.0 0.0 0.0) _asplayer_1 450.0
    (:`OnSuccess`
      (if (> (`self.Health`) 0.0)
        (`|SpawnActorFromClass` "/Game/Blueprints/Bullet.Bullet_C" (`KismetMathLibrary.MakeTransform` (+ (`SceneComponent.K2_GetComponentLocation` (`self.FirePoint`)) (`KismetMathLibrary.GreaterGreater_VectorRotator` (`self.GunOffset`) (`SceneComponent.K2_GetComponentRotation` (`self.Gun`)))) (`KismetMathLibrary.FindLookAtRotation` (`self.K2_GetActorLocation`) (`self.K2_GetActorLocation` (cast `/Game/Blueprints/Player1` (`GameplayStatics.GetPlayerCharacter` 0) :!pure true)))) "Undefined" "OverrideRootScale" null null)
        (`GameplayStatics.PlaySoundAtLocation` "/Game/Audio/Gunshot2.Gunshot2" (`self.K2_GetActorLocation`) (struct) 1.0 1.0 0.0 null null null)
        (if (not (`self.GrenadeLaunched`))
          (`|SpawnActorFromClass` "/Game/Blueprints/Grenade.Grenade_C" (`KismetMathLibrary.MakeTransform` (+ (`SceneComponent.K2_GetComponentLocation` (`self.LaunchPoint`)) (`KismetMathLibrary.GreaterGreater_VectorRotator` (`self.GunOffset`) (`SceneComponent.K2_GetComponentRotation` (`self.Gun`)))) (`KismetMathLibrary.FindLookAtRotation` (`self.K2_GetActorLocation`) (`self.K2_GetActorLocation` (cast `/Game/Blueprints/Player1` (`GameplayStatics.GetPlayerCharacter` 0) :!pure true)))) "Undefined" "OverrideRootScale" null null)
          (set `self.GrenadeLaunched` true)
          (`KismetSystemLibrary.Delay` 3.0)
          (set `self.GrenadeLaunched` false))))))

(fn `UserConstructionScript`)