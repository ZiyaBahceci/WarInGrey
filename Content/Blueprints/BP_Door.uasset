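; BP_Door is a key-locked door that the player opens and closes with F while inside its trigger.
; DoorTrigger overlap enables or disables input on the actor.
; If BP_Player1 has the key, a toggle plays or reverses a timeline that rotates the root in yaw by Angle, with sweep.
; Otherwise it sets the player's hint text and, only once, shows a timed WBP_Intercom widget.
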(event `self.DoorTrigger.OnComponentBeginOverlap`
  (params (OverlappedComponent :type "PrimitiveComponent Object Reference") (OtherActor :type "Actor Object Reference") (OtherComp :type "PrimitiveComponent Object Reference") (OtherBodyIndex :type Integer) (bFromSweep :type Boolean) (SweepResult :type "HitResult Structure (by ref)"))
  ;[1 1 1] Door Proximity
  (`self.EnableInput` (`GameplayStatics.GetPlayerController` 0)))

(event `self.DoorTrigger.OnComponentEndOverlap`
  (params (OverlappedComponent :type "PrimitiveComponent Object Reference") (OtherActor :type "Actor Object Reference") (OtherComp :type "PrimitiveComponent Object Reference") (OtherBodyIndex :type Integer))
  ;[1 1 1] Door Proximity
  (`self.DisableInput` (`GameplayStatics.GetPlayerController` 0)))

(event `Key|F`
  (params (Key :type "Key Structure"))
  ;[1 1 1] Check if player has key
  (:`Pressed`
    (bind _asplayer_1 (cast `/Game/Blueprints/BP_Player1` (`GameplayStatics.GetPlayerCharacter` 0)))
    (if (`/Game/Blueprints/BP_Player1.HasKey` _asplayer_1)
      ;[1 1 1] Open/Close Door
      (if (`self.InteractState`)
        (set `self.InteractState` false)
        (bind (_direction _doorinterpolation) (`Timeline|DoorTimeline` :!via `Reverse` :!label _label)
          (:`Update`
            (`SceneComponent.K2_SetRelativeRotation` (`self.DefaultSceneRoot`) (`KismetMathLibrary.MakeRotator` 0.0 0.0 (* (`self.Angle`) _doorinterpolation)) true false)))
        (else
          (set `self.InteractState` true)
          (goto _label)))
      (else
        ;[1 1 1] If player doesn't have the key, create hint widget for 5 seconds.
        (bind _asplayer_1_2 (cast `/Game/Blueprints/BP_Player1` (`GameplayStatics.GetPlayerCharacter` 0)))
        (set `/Game/Blueprints/BP_Player1.HintText` "Door is locked. Key is most likely in the warehouse." _asplayer_1_2)
        (`/Engine/EditorBlueprintResources/StandardMacros.DoOnce` false
          (:`Completed`
            (bind _returnvalue (`|CreateWidget` "/Game/UI/HUD/WBP_Intercom.WBP_Intercom_C" (`GameplayStatics.GetPlayerController` 0)))
            (`UserWidget.AddToViewport` _returnvalue 0)
            (`KismetSystemLibrary.Delay` 5.0)
            (`Widget.RemoveFromParent` _returnvalue)))))))

(fn `UserConstructionScript`)