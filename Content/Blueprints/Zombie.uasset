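; Zombie enemy actor that takes damage, dies and strikes the player with a melee attack.
; Any damage lowers Health; at zero, DoOnce gates enable Body physics and play a death sound before a delayed destroy.
; Attack swings the right arm with chained MoveComponentTo calls, then damages the player if their capsule overlaps the Sphere.
; A score increment on the game instance exists but is unconnected.
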(event `self.ReceiveAnyDamage`
  (params (Damage :type "Float (single-precision)") (DamageType :type "DamageType Object Reference") (InstigatedBy :type "Controller Object Reference") (DamageCauser :type "Actor Object Reference"))
  ;[1 1 1] Health and Death
  (`GameplayStatics.PlaySoundAtLocation` "/Game/Audio/Hit.Hit" (`self.K2_GetActorLocation`) (struct) 1.0 1.0 0.0 null null null)
  (set `self.Health` (- (`self.Health`) Damage))
  (if (<= (`self.Health`) 0.0)
    (`/Engine/EditorBlueprintResources/StandardMacros.DoOnce` false
      (:`Completed`
        (`PrimitiveComponent.SetSimulatePhysics` (`self.Body`) true)
        (`/Engine/EditorBlueprintResources/StandardMacros.DoOnce` false
          (:`Completed`
            (`GameplayStatics.PlaySoundAtLocation` "/Game/Audio/ZombieDeath.ZombieDeath" (`self.K2_GetActorLocation`) (struct) 1.0 1.0 0.0 null null null)
            (`KismetSystemLibrary.Delay` 2.0)
            (`self.K2_DestroyActor`)))))))

(event `Attack`
  (bind _rightarmupper (`self.RightArmUpper`))
  ;[1 1 1] Attacking
  (`GameplayStatics.PlaySoundAtLocation` "/Game/Audio/ZombieAttackCue.ZombieAttackCue" (`self.K2_GetActorLocation`) (struct) 1.0 1.0 0.0 null null null)
  (`KismetSystemLibrary.MoveComponentTo` _rightarmupper (42.0 40.0 63.0) (struct :`Pitch` -39.0 :`Yaw` 9.0 :`Roll` 1.0) true true 0.4)
  (`KismetSystemLibrary.MoveComponentTo` _rightarmupper (42.0 40.0 45.0) (struct :`Pitch` -77.0 :`Yaw` 40.0 :`Roll` -34.0) true true 0.1)
  (bind _asplayer_1 (cast `/Game/Blueprints/Player1` (`GameplayStatics.GetPlayerCharacter` 0)))
  (if (`PrimitiveComponent.IsOverlappingComponent` (`Character.CapsuleComponent` (`GameplayStatics.GetPlayerCharacter` 0)) (`self.Sphere`))
    (`GameplayStatics.ApplyDamage` _asplayer_1 20.0)))

(fn `UserConstructionScript`)