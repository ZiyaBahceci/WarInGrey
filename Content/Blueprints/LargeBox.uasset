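; LargeBox is a box that becomes pushable only while something overlaps one of its two collision volumes, XAxisCollision or YAxisCollision.
; Each volume turns physics simulation on at begin overlap and off at end overlap, with no check on the overlapping actor or the other volume.
; Both volumes run identical logic, so the graph itself applies no axis-specific constraint.
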(event `self.X Axis Collision.OnComponentBeginOverlap`
  (params (OverlappedComponent :type "PrimitiveComponent Object Reference") (OtherActor :type "Actor Object Reference") (OtherComp :type "PrimitiveComponent Object Reference") (OtherBodyIndex :type Integer) (bFromSweep :type Boolean) (SweepResult :type "HitResult Structure (by ref)"))
  ;[1 1 1] Make box pushable on  X axis
  (`PrimitiveComponent.SetSimulatePhysics` (`self.LargeBox`) true))

(event `self.X Axis Collision.OnComponentEndOverlap`
  (params (OverlappedComponent :type "PrimitiveComponent Object Reference") (OtherActor :type "Actor Object Reference") (OtherComp :type "PrimitiveComponent Object Reference") (OtherBodyIndex :type Integer))
  ;[1 1 1] Make box pushable on  X axis
  (`PrimitiveComponent.SetSimulatePhysics` (`self.LargeBox`) false))

(event `self.Y Axis Collision.OnComponentBeginOverlap`
  (params (OverlappedComponent :type "PrimitiveComponent Object Reference") (OtherActor :type "Actor Object Reference") (OtherComp :type "PrimitiveComponent Object Reference") (OtherBodyIndex :type Integer) (bFromSweep :type Boolean) (SweepResult :type "HitResult Structure (by ref)"))
  ;[1 1 1] Make box pushable on  Y axis
  (`PrimitiveComponent.SetSimulatePhysics` (`self.LargeBox`) true))

(event `self.Y Axis Collision.OnComponentEndOverlap`
  (params (OverlappedComponent :type "PrimitiveComponent Object Reference") (OtherActor :type "Actor Object Reference") (OtherComp :type "PrimitiveComponent Object Reference") (OtherBodyIndex :type Integer))
  ;[1 1 1] Make box pushable on  Y axis
  (`PrimitiveComponent.SetSimulatePhysics` (`self.LargeBox`) false))

(fn `UserConstructionScript`)