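; Objective trigger volume that starts the "Kill the Lords of War officer" boss fight when Player1 overlaps its Box.
; On overlap it sets the player's objective text, swaps the factory soundtrack for the bossfight track, and moves the objective marker via WiGGameInstance.
; It also saves a checkpoint in the game instance with a respawn location and area-state flags, then destroys itself so it fires only once.
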(event `self.Box.OnComponentBeginOverlap`
  (params (OverlappedComponent :type "PrimitiveComponent Object Reference") (OtherActor :type "Actor Object Reference") (OtherComp :type "PrimitiveComponent Object Reference") (OtherBodyIndex :type Integer) (bFromSweep :type Boolean) (SweepResult :type "HitResult Structure (by ref)"))
  ;[1 1 1] Set Objective
  (bind _asplayer_1 (cast `/Game/Blueprints/Player1` OtherActor))
  (set `/Game/Blueprints/Player1.ObjectiveText` "Kill the Lords of War officer" _asplayer_1)
  ;[1 1 1] Change Soundtrack
  (bind _asplayer_1_2 (cast `/Game/Blueprints/Player1` (`GameplayStatics.GetPlayerCharacter` 0)))
  (`AudioComponent.Stop` (`/Game/Blueprints/Player1.SoundtrackFactory` _asplayer_1_2))
  (`AudioComponent.Play` (`/Game/Blueprints/Player1.SoundtrackBossfight` _asplayer_1_2) 0.0)
  ;[1 1 1] Set Marker Location
  (bind _aswi_ggame_instance (cast `/Game/GameModes/WiGGameInstance` (`GameplayStatics.GetGameInstance`)))
  (set `/Game/GameModes/WiGGameInstance.MarkerLocation` (7044.0 1680.0 70.0) _aswi_ggame_instance)
  ;[1 1 1] Save Checkpoint
  (bind _aswi_ggame_instance_2 (cast `/Game/GameModes/WiGGameInstance` (`GameplayStatics.GetGameInstance`)))
  (set `/Game/GameModes/WiGGameInstance.CheckpointSaved` true _aswi_ggame_instance_2)
  (set `/Game/GameModes/WiGGameInstance.SavedLocation` (8356.0 736.0 1871.0) _aswi_ggame_instance_2)
  (set `/Game/GameModes/WiGGameInstance.InSecurityRoom` true _aswi_ggame_instance_2)
  (set `/Game/GameModes/WiGGameInstance.GateClosed` true _aswi_ggame_instance_2)
  (set `/Game/GameModes/WiGGameInstance.InCompound` true _aswi_ggame_instance_2)
  (`self.K2_DestroyActor`))

(fn `UserConstructionScript`)