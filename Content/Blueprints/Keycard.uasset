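; Keycard pickup actor that gives the player the key needed to interact with the door.
; The first Box overlap sets HasKey and the hint text on the Player1 character, without checking which actor overlapped.
; It then destroys its mesh, text and trigger components rather than the actor, and shows a Hint widget for five seconds.
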(event `self.Box.OnComponentBeginOverlap`
  (params (OverlappedComponent :type "PrimitiveComponent Object Reference") (OtherActor :type "Actor Object Reference") (OtherComp :type "PrimitiveComponent Object Reference") (OtherBodyIndex :type Integer) (bFromSweep :type Boolean) (SweepResult :type "HitResult Structure (by ref)"))
  (bind _asplayer_1 (cast `/Game/Blueprints/Player1` (`GameplayStatics.GetPlayerCharacter` 0)))
  (`/Engine/EditorBlueprintResources/StandardMacros.DoOnce` false
    (:`Completed`
      ;[1 1 1] This boolean lets the player interact with the door
      (set `/Game/Blueprints/Player1.HasKey` true _asplayer_1)
      ;[1 1 1] 5-Second "Keycard Acquired" information
      (bind _asplayer_1_2 (cast `/Game/Blueprints/Player1` (`GameplayStatics.GetPlayerCharacter` 0)))
      (set `/Game/Blueprints/Player1.HintText` "Keycard acquired." _asplayer_1_2)
      (`ActorComponent.K2_DestroyComponent` (`self.Cube`))
      (`ActorComponent.K2_DestroyComponent` (`self.TextRender1`))
      (`ActorComponent.K2_DestroyComponent` (`self.TextRender`))
      (`ActorComponent.K2_DestroyComponent` (`self.Box`))
      (bind _returnvalue (`|CreateWidget` "/Game/UI/Hint.Hint_C" (`GameplayStatics.GetPlayerController` 0)))
      (`UserWidget.AddToViewport` _returnvalue 0)
      (`KismetSystemLibrary.Delay` 5.0)
      (`Widget.RemoveFromParent` _returnvalue))))

(fn `UserConstructionScript`)