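; Gun pickup actor that arms the player on box overlap and records the pickup in the game instance for saves.
; Overlap hides the rifle, flags the save before checking for Player1, then reveals the player's gun and arms and adds the ammo counter and controls hint.
; Tick destroys the actor once GunPickedUp is set, covering checkpoint loads but also preempting the delayed hint removal.
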(event `self.Box.OnComponentBeginOverlap`
  (params (OverlappedComponent :type "PrimitiveComponent Object Reference") (OtherActor :type "Actor Object Reference") (OtherComp :type "PrimitiveComponent Object Reference") (OtherBodyIndex :type Integer) (bFromSweep :type Boolean) (SweepResult :type "HitResult Structure (by ref)"))
  ;[1 1 1] Hide Gun Upon Pickup
  (`SceneComponent.SetVisibility` (`self.AssaultRifle`) false false)
  ;[1 1 1] For Saves
  (set `/Game/GameModes/WiGGameInstance.PickedUpGun` true (cast `/Game/GameModes/WiGGameInstance` (`GameplayStatics.GetGameInstance`) :!pure true))
  ;[1 1 1] Make Gun and Hands Visible For Player
  (bind _asplayer_1 (cast `/Game/Blueprints/Player1` OtherActor))
  (`SceneComponent.SetVisibility` (`/Game/Blueprints/Player1.Gun` _asplayer_1) true false)
  (`SceneComponent.SetVisibility` (`/Game/Blueprints/Player1.LeftArm` _asplayer_1) true false)
  (`SceneComponent.SetVisibility` (`/Game/Blueprints/Player1.RightArm` _asplayer_1) true false)
  (`SceneComponent.SetVisibility` (`/Game/Blueprints/Player1.RightHand` _asplayer_1) true false)
  (`SceneComponent.SetVisibility` (`/Game/Blueprints/Player1.LeftHand` _asplayer_1) true false)
  ;[1 1 1] Ammo Counter Widget
  (bind _returnvalue (`|CreateWidget` "/Game/UI/AmmoCounter.AmmoCounter_C" (cast `PlayerController` (`Pawn.GetController` (`GameplayStatics.GetPlayerCharacter` 0)) :!pure true)))
  (`UserWidget.AddToViewport` _returnvalue 0)
  ;[1 1 1] Disable gun existing if player loaded checkpoint and already has gun
  (set `/Game/Blueprints/Player1.GunPickedUp` true _asplayer_1)
  ;[1 1 1] Gun Hint
  (set `/Game/Blueprints/Player1.HintText` "Use Left Mouse to shoot, Right Mouse to aim, Middle Mouse for alt. fire, Ctrl to Melee." _asplayer_1)
  (`/Engine/EditorBlueprintResources/StandardMacros.DoOnce` false
    (:`Completed`
      (bind _returnvalue_2 (`|CreateWidget` "/Game/UI/Hint.Hint_C" (`GameplayStatics.GetPlayerController` 0)))
      (`UserWidget.AddToViewport` _returnvalue_2 0)
      (`KismetSystemLibrary.Delay` 5.0)
      (`Widget.RemoveFromParent` _returnvalue_2)
      (`self.K2_DestroyActor`))))

(event `self.ReceiveTick`
  (params (DeltaSeconds :type "Float (single-precision)"))
  ;[1 1 1] If gun picked up, destroy actor
  (if (`/Game/Blueprints/Player1.GunPickedUp` (cast `/Game/Blueprints/Player1` (`GameplayStatics.GetPlayerCharacter` 0) :!pure true))
    (`self.K2_DestroyActor`)))

(fn `UserConstructionScript`)