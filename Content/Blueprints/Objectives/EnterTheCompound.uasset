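; EnterTheCompound is a one-shot trigger volume that advances the mission objective to entering the compound.
; When BP_Player1 overlaps its box, it sets the player's objective text and moves the marker location stored in WiGGameInstance.
; It also flags a checkpoint in the game instance at its own root location, then destroys itself.
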(event `self.Box.OnComponentBeginOverlap`
  (params (OverlappedComponent :type "PrimitiveComponent Object Reference") (OtherActor :type "Actor Object Reference") (OtherComp :type "PrimitiveComponent Object Reference") (OtherBodyIndex :type Integer) (bFromSweep :type Boolean) (SweepResult :type "HitResult Structure (by ref)"))
  ;[1 1 1] Set Objective
  (bind _asplayer_1 (cast `/Game/Blueprints/BP_Player1` OtherActor))
  (set `/Game/Blueprints/BP_Player1.ObjectiveText` "Make your way into the compound" _asplayer_1)
  ;[1 1 1] Set Marker Location
  (bind _aswi_ggame_instance (cast `/Game/GameModes/WiGGameInstance` (`GameplayStatics.GetGameInstance`)))
  (set `/Game/GameModes/WiGGameInstance.MarkerLocation` (5780.0 730.0 1030.0) _aswi_ggame_instance)
  ;[1 1 1] Save Checkpoint
  (bind _aswi_ggame_instance_2 (cast `/Game/GameModes/WiGGameInstance` (`GameplayStatics.GetGameInstance`)))
  (set `/Game/GameModes/WiGGameInstance.CheckpointSaved` true _aswi_ggame_instance_2)
  (set `/Game/GameModes/WiGGameInstance.SavedLocation` (`SceneComponent.K2_GetComponentLocation` (`self.DefaultSceneRoot`)) _aswi_ggame_instance_2)
  (`self.K2_DestroyActor`))

(fn `UserConstructionScript`)