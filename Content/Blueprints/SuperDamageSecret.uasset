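; SuperDamageSecret is a hidden pickup that permanently boosts the player's gun damage when its Box is first overlapped.
; The one-shot overlap plays a sound, sets Player1's GunDamage, adds to the game instance's secret count and score, and removes the TextRender.
; It then sets the player's HintText, shows a Hint widget for five seconds and destroys itself.
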(event `self.Box.OnComponentBeginOverlap`
  (params (OverlappedComponent :type "PrimitiveComponent Object Reference") (OtherActor :type "Actor Object Reference") (OtherComp :type "PrimitiveComponent Object Reference") (OtherBodyIndex :type Integer) (bFromSweep :type Boolean) (SweepResult :type "HitResult Structure (by ref)"))
  (bind _returnvalue (`GameplayStatics.GetPlayerCharacter` 0))
  (`/Engine/EditorBlueprintResources/StandardMacros.DoOnce` false
    (:`Completed`
      (`GameplayStatics.PlaySound2D` "/Game/Audio/SecretFound.SecretFound" 1.0 1.0 0.0 null null)
      ;[1 1 1] Increase weapon damage
      (bind _asplayer_1 (cast `/Game/Blueprints/Player1` _returnvalue))
      (set `/Game/Blueprints/Player1.GunDamage` 25.0 _asplayer_1)
      ;[1 1 1] Increase score and secret count
      (bind _aswi_ggame_instance (cast `/Game/GameModes/WiGGameInstance` (`GameplayStatics.GetGameInstance`)))
      (set `/Game/GameModes/WiGGameInstance.SecretsFound` (+ (`/Game/GameModes/WiGGameInstance.SecretsFound` _aswi_ggame_instance) 1.0) _aswi_ggame_instance)
      (set `/Game/GameModes/WiGGameInstance.Score` (+ (`/Game/GameModes/WiGGameInstance.Score` _aswi_ggame_instance) 1000.0) _aswi_ggame_instance)
      ;[1 1 1] Destroy interactable part of the object
      (`ActorComponent.K2_DestroyComponent` (`self.TextRender`))
      ;[1 1 1] 5-second information widget
      (bind _asplayer_1_2 (cast `/Game/Blueprints/Player1` _returnvalue))
      (set `/Game/Blueprints/Player1.HintText` "Secret found! Damage increased." _asplayer_1_2)
      (`/Engine/EditorBlueprintResources/StandardMacros.DoOnce` false
        (:`Completed`
          (bind _returnvalue_2 (`|CreateWidget` "/Game/UI/Hint.Hint_C" (`GameplayStatics.GetPlayerController` 0)))
          (`UserWidget.AddToViewport` _returnvalue_2 0)
          (`KismetSystemLibrary.Delay` 5.0)
          (`Widget.RemoveFromParent` _returnvalue_2)
          (`self.K2_DestroyActor`))))))

(fn `UserConstructionScript`)